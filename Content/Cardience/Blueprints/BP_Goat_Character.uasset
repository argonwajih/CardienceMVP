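; Goat unit Blueprint for Cardience that supplies goat-specific animations and attack behavior.
; BeginPlay runs Initialise and sets the root to a 90-degree rotation for opponent units.
; LaunchAttack, upon reaching the target, locks movement, calls Attack, plays the looping attack animation and clears the reached flag; otherwise it unlocks movement.
; Idle, move and attack functions play looping clips directly on the skeletal mesh, while the hit animation function is empty.
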(event EventBeginPlay
  (CallFunction|Initialise)
  (if (Variables|Default|GetIsOpponent)
    (Transformation|SetRelativeRotation (Variables|Default|GetDefaultSceneRoot) "0,90.000000, 0" false false)))

(fn ConstructionScript)

(fn PlayAttackAnimation
  (Components|Animation|PlayAnimation (Variables|Default|GetSkeletalMesh) "/Game/Cardience/CardienceCharacters/Goat/GoatAttackAnimFinalFbx_Anim.GoatAttackAnimFinalFbx_Anim" true))

(fn PlayHitAnimation)

(fn LaunchAttack
  (if (Variables|Default|GetHasReachedTarget?)
    (CallFunction|ManageMovementLock true)
    (CallFunction|Attack)
    (CallFunction|PlayAttackAnimation)
    (Variables|Default|SetHasReachedTarget? false)
    (else
      (CallFunction|ManageMovementLock false))))

(fn PlayIdleAnimation
  (Components|Animation|PlayAnimation (Variables|Default|GetSkeletalMesh) "/Game/Cardience/CardienceCharacters/Goat/GoatIdleFbxFinal_Anim.GoatIdleFbxFinal_Anim" true))

(fn PlayMoveAnimation
  (Components|Animation|PlayAnimation (Variables|Default|GetSkeletalMesh) "/Game/Cardience/CardienceCharacters/Goat/GoatRunAnimFBXFinal__1__Anim.GoatRunAnimFBXFinal__1__Anim" true))