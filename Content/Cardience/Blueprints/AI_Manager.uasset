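; AI manager for a team battle that tracks player and opponent characters, assigns targets and handles game over.
; SetTargets pairs same-class characters across teams, then starts the fight by clearing destroyable characters, revealing the player's team and looping all level sequences.
; FindNewTarget picks a living enemy of equal priority, falling back to highest priority, and relaunches the attack.
; Death events update rosters and show GameOver; opponent spawning is unwired.
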(event Custom|PopulateSpawnablePoints
  (Variables|Default|SetCurrentFreePlacements (Utilities|Array|MakeArray (Variables|Default|GetScene4) (Variables|Default|GetScene1) (Variables|Default|GetScene2) (Variables|Default|GetScene3) (Variables|Default|GetScene) (Variables|Default|GetScene5) (Variables|Default|GetScene6) (Variables|Default|GetScene7) (Variables|Default|GetScene8))))

(event Custom|SetTargets
  (for _array_element (Variables|Default|GetOpponentCharacters)
    (for _array_element_2 (Variables|Default|GetPlayerCharacters)
      (if (== (Utilities|GetClass _array_element) (Utilities|GetClass _array_element_2))
        (Variables|/Game/Cardience/Blueprints/DummyCharacter.DummyCharacter_C|SetOpponentTarget _array_element _array_element_2)
        (Variables|/Game/Cardience/Blueprints/DummyCharacter.DummyCharacter_C|SetOpponentTarget _array_element_2 _array_element))))
  (for _array_element_3 (Variables|Default|GetOpponentCharacters)
    _)
  (for _array_element_4 (Variables|Default|GetPlayerCharacters)
    _)
  (CallFunction|StartFight))

(event Custom|AddDestroyableCharacter
  (params (Character :type Dummy%20Character%20Object%20Reference))
  (Utilities|Array|Add (Variables|Default|GetDestroyableCharacters) Character))

(event Custom|StartFight
  (CallFunction|DestroyAllCharacters)
  (CallFunction|ManagePlayerCharactersVisibility false)
  (bind _outactors (Actor|GetAllActorsOfClass "/Script/LevelSequence.LevelSequenceActor"))
  (for _array_element _outactors
    (Class|MovieSceneSequencePlayer|PlayLooping (Variables|/Script/LevelSequence.LevelSequenceActor|GetSequencePlayer _array_element) -1)))

(event Custom|FindNewTarget
  (params (Character :type Dummy%20Character%20Object%20Reference))
  (if (Variables|/Game/Cardience/Blueprints/DummyCharacter.DummyCharacter_C|GetIsOpponent Character)
    (bind _opponenttarget (CallFunction|FindTargett Character (Variables|Default|GetPlayerCharacters)))
    (Variables|/Game/Cardience/Blueprints/DummyCharacter.DummyCharacter_C|SetOpponentTarget Character _opponenttarget)
    (Default|LaunchAttack Character)
    (else
      (bind _opponenttarget_2 (CallFunction|FindTargett Character (Variables|Default|GetOpponentCharacters)))
      (bind _output_get (Variables|/Game/Cardience/Blueprints/DummyCharacter.DummyCharacter_C|SetOpponentTarget Character _opponenttarget_2))
      (Default|LaunchAttack Character))))

(event Custom|OnCharac_Dead
  (params (Character :type Dummy%20Character%20Object%20Reference))
  (if (Variables|/Game/Cardience/Blueprints/DummyCharacter.DummyCharacter_C|GetIsOpponent Character)
    (Utilities|Array|RemoveItem (Variables|Default|GetOpponentCharacters) Character)
    (else
      (Utilities|Array|RemoveItem (Variables|Default|GetPlayerCharacters) 0)))
  (if (== (Utilities|Array|Length (Variables|Default|GetOpponentCharacters)) 0)
    (Default|CallOnGameOver true)
    (Variables|Default|SetDidYouWin? true)
    (elif (== (Utilities|Array|Length (Variables|Default|GetPlayerCharacters)) 0)
      (Default|CallOnGameOver false)
      (Variables|Default|SetDidYouWin? false)
      (else
        (Default|CallOnGameOver true)
        (Variables|Default|SetDidYouWin? true))))
  (bind _returnvalue (UserInterface|CreateWidget "/Game/Cardience/Blueprints/UI/GameOver.GameOver_C"))
  (UserInterface|Viewport|AddtoViewport _returnvalue 0))

(event EventBeginPlay
  (EventDispatchers|BindEventtoOnCharacterDead (delegate Custom|OnCharac_Dead))
  (CallFunction|ManagePlayerCharactersVisibility true)
  (CallFunction|PopulateSpawnablePoints))

(fn ConstructionScript)

(fn GetPlacementPosition
  (bind _currentfreeplacements (Variables|Default|GetCurrentFreePlacements))
  (Variables|Default|SetRand (Math|Random|RandomInteger (- (Utilities|Array|Length _currentfreeplacements) 1)))
  (LocalVariables|SetPosition (Transformation|GetWorldLocation (Utilities|Array|Get(acopy) _currentfreeplacements (Variables|Default|GetRand))))
  (Utilities|Array|RemoveIndex (Variables|Default|GetCurrentFreePlacements) (Variables|Default|GetRand))
  (return (LocalVariables|GetPosition)))

(fn DestroyAllCharacters
  (bind _destroyablecharacters (Variables|Default|GetDestroyableCharacters))
  (for _index (range 0 (- (Utilities|Array|Length (Variables|Default|GetDestroyableCharacters)) 1))
    (Actor|DestroyActor (Utilities|Array|Get(acopy) _destroyablecharacters _index)))
  (Utilities|Array|Clear _destroyablecharacters))

(fn FindTargett
  (params (Character :type Dummy%20Character%20Object%20Reference) (OpponentsListToFindTargetFrom :type Array%20of%20Dummy%20Character%20Object%20References))
  (for _array_element OpponentsListToFindTargetFrom
    (Utilities|IsValid _array_element
      (:Is%20Valid
        (if (and (== (Variables|/Game/Cardience/Blueprints/DummyCharacter.DummyCharacter_C|GetPriority _array_element) (Variables|/Game/Cardience/Blueprints/DummyCharacter.DummyCharacter_C|GetPriority Character)) (> (Variables|/Game/Cardience/Blueprints/DummyCharacter.DummyCharacter_C|GetHealth _array_element) 0))
          (return _array_element)))))
  (for _array_element_2 OpponentsListToFindTargetFrom
    (Utilities|IsValid _array_element_2
      (:Is%20Valid
        (if (and (> (Variables|/Game/Cardience/Blueprints/DummyCharacter.DummyCharacter_C|GetPriority _array_element_2) (LocalVariables|GetHigestPriority)) (> (Variables|/Game/Cardience/Blueprints/DummyCharacter.DummyCharacter_C|GetHealth _array_element_2) 0))
          (LocalVariables|SetHigestPriority (Variables|/Game/Cardience/Blueprints/DummyCharacter.DummyCharacter_C|GetPriority _array_element_2))))))
  (for _array_element_3 OpponentsListToFindTargetFrom
    (Utilities|IsValid _array_element_3
      (:Is%20Valid
        (if (and (== (Variables|/Game/Cardience/Blueprints/DummyCharacter.DummyCharacter_C|GetPriority _array_element_3) (LocalVariables|GetHigestPriority)) (> (Variables|/Game/Cardience/Blueprints/DummyCharacter.DummyCharacter_C|GetHealth _array_element_3) 0))
          (return _array_element_3))))))

(fn ManagePlayerCharactersVisibility
  (params (Hidden? :type Boolean))
  (for _array_element (Variables|Default|GetPlayerCharacters)
    (Rendering|SetActorHiddenInGame _array_element Hidden?)))