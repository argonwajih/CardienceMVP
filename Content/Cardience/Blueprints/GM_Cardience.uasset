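; GM_Cardience, by its name the game mode for Cardience, provides a screen-switching helper for the UI.
; OpenUI removes all widgets, then creates the given widget class if valid, adds it to the viewport and returns it.
; The event graph holds only an unconnected copy of that logic, and the construction script is empty.
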(fn ConstructionScript)

(fn OpenUI
  (params (UI :type UI%20Main%20Class%20Reference))
  (Viewport|RemoveAllWidgets)
  (if (Utilities|IsValidClass UI)
    (bind _returnvalue (UserInterface|CreateWidget UI))
    (UserInterface|Viewport|AddtoViewport _returnvalue 0)
    (return _returnvalue)))