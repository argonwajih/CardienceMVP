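; DummyCharacter is an AI-driven combatant that faces and moves straight toward its OpponentTarget each tick, then calls LaunchAttack within stopping distance.
; A separate Attack event repeatedly spawns target-assigned bullets at random intervals.
; GetAttackHit reduces health and reports death to AI_Manager before destroying the actor.
; LaunchAttack and animation functions are empty stubs, and the handlers for retargeting and game-over locking have their manager bindings disconnected.
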(event Custom|OnCharacterDead
  (params (Character :type Dummy%20Character%20Object%20Reference))
  (if (== Character (Variables|Default|GetOpponentTarget))
    (Default|FindNewTarget (Utilities|Array|Get(acopy) (stale Custom|Initialise _outactors)) self)))

(event Custom|Initialise
  (bind _outactors (Actor|GetAllActorsOfClass "/Game/Cardience/Blueprints/AI_Manager.AI_Manager_C")))

(event Custom|OnGameOver
  (params (DidYouWin? :type Boolean))
  (CallFunction|ManageMovementLock true)
  (if DidYouWin?
    _))

(event Custom|Attack
  (bind _returnvalue (Game|SpawnActorfromClass "/Game/Cardience/Blueprints/Bullet.Bullet_C" (Math|Transform|MakeTransform (Transformation|GetActorLocation) "0, 0, 0" "1,1,1") "Undefined" 0 5e+02 10 0 :!label _label))
  (Variables|/Game/Cardience/Blueprints/Bullet.Bullet_C|SetTarget _returnvalue (Variables|Default|GetOpponentTarget))
  (Utilities|FlowControl|Delay (Math|Random|RandomFloatinRange 1.0 5.0))
  (goto _label))

(event EventBeginPlay
  (CallFunction|Initialise))

(event EventTick
  (params (DeltaSeconds :type Float%20%28single-precision%29))
  (Utilities|FlowControl|Sequence
    (:then_0
      (Utilities|IsValid (Variables|Default|GetOpponentTarget)
        (:Is%20Valid
          (Transformation|SetActorRotation (Math|Rotator|FindLookatRotation (Transformation|GetActorLocation) (Transformation|GetActorLocation (Variables|Default|GetOpponentTarget)))))))
    (:then_1
      (CallFunction|MoveTowardsTarget DeltaSeconds 75.0 (Variables|Default|GetSpeed)))))

(fn ConstructionScript)

(fn MoveTowardsTarget
  (params (Delta :type Float%20%28single-precision%29) (StoppingDistance :type Float%20%28single-precision%29) (Speed :type Float%20%28single-precision%29))
  (if (and (Variables|Default|GetIsMoveableCharacter) (Variables|Default|GetCanMove))
    (Utilities|IsValid (Variables|Default|GetOpponentTarget)
      (:Is%20Valid
        (LocalVariables|SetRemainingDistance (Math|Vector|Distance(Vector) (Transformation|GetActorLocation (Variables|Default|GetOpponentTarget)) (Transformation|GetActorLocation)))
        (if (>= (LocalVariables|GetRemainingDistance) StoppingDistance)
          (bind _output_get (LocalVariables|SetDirection (Math|Vector|Normalize (- (Transformation|GetActorLocation (Variables|Default|GetOpponentTarget)) (Transformation|GetActorLocation)))))
          (Transformation|SetActorLocation (+ (Transformation|GetActorLocation) (* _output_get (* Speed Delta))) false false)
          (else
            (Variables|Default|SetHasReachedTarget? true)
            (CallFunction|LaunchAttack)))))))

(fn GetAttackHit
  (params (Damage :type Integer))
  (bind _output_get (Variables|Default|SetHealth (- (Variables|Default|GetHealth) Damage)))
  (if (<= _output_get 0)
    (bind _outactors (Actor|GetAllActorsOfClass "/Game/Cardience/Blueprints/AI_Manager.AI_Manager_C"))
    (Default|CallOnCharacterDead (Utilities|Array|Get(acopy) _outactors) self)
    (Actor|DestroyActor)
    (else
      (CallFunction|PlayHitAnimation))))

(fn PlayAttackAnimation)

(fn PlayHitAnimation)

(fn PlayIdleAnimation)

(fn PlayMoveAnimation)

(fn LaunchAttack)

(fn ManageMovementLock
  (params (IsLocked? :type Boolean))
  (bind _output_get (Variables|Default|SetCanMove (not IsLocked?)))
  (if _output_get
    (CallFunction|PlayMoveAnimation)
    (else
      (CallFunction|PlayIdleAnimation))))