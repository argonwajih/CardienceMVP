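; Female character Blueprint for Cardience that supplies skeletal mesh animation for attacks.
; BeginPlay calls Initialise, then checks IsOpponent with no action wired to it.
; LaunchAttack locks movement, calls Attack and plays a looping shooting animation.
; PlayHitAnimation is empty, with its looping punch-reaction node left disconnected, as is a root rotation node in the event graph.
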(event EventBeginPlay
  (CallFunction|Initialise)
  (if (Variables|Default|GetIsOpponent)
    _))

(fn ConstructionScript)

(fn PlayAttackAnimation
  (Components|Animation|PlayAnimation (Variables|Default|GetSkeletalMesh) "/Game/Cardience/CardienceCharacters/girl/v1/shooting/Female_Shooting_Animations_Anim.Female_Shooting_Animations_Anim" true))

(fn PlayHitAnimation)

(fn LaunchAttack
  (CallFunction|ManageMovementLock true)
  (CallFunction|Attack)
  (CallFunction|PlayAttackAnimation))