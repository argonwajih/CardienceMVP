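; Homing bullet actor that chases a Target and deals damage on arrival.
; Each tick it rotates to face the target and steps toward it at Speed via MoveTowardsTarget, without sweep or collision checks.
; Once within a short stopping distance it calls GetAttackHit with its Damage on the target and destroys itself.
; It also destroys itself if the target becomes invalid.
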(event EventBeginPlay)

(event Collision|EventActorBeginOverlap
  (params (OtherActor :type Actor%20Object%20Reference)))

(event EventTick
  (params (DeltaSeconds :type Float%20%28single-precision%29))
  (Utilities|IsValid (Variables|Default|GetTarget)
    (:Is%20Valid
      (Transformation|SetActorRotation (Math|Rotator|FindLookatRotation (Transformation|GetActorLocation) (Transformation|GetActorLocation (Variables|Default|GetTarget))))
      (CallFunction|MoveTowardsTarget DeltaSeconds 5e+01 (Variables|Default|GetSpeed)))
    (:Is%20Not%20Valid
      (Actor|DestroyActor))))

(fn ConstructionScript)

(fn MoveTowardsTarget
  (params (Delta :type Float%20%28single-precision%29) (StoppingDistance :type Float%20%28single-precision%29) (Speed :type Float%20%28single-precision%29))
  (LocalVariables|SetRemainingDistance (Math|Vector|Distance(Vector) (Transformation|GetActorLocation (Variables|Default|GetTarget)) (Transformation|GetActorLocation)))
  (if (>= (LocalVariables|GetRemainingDistance) StoppingDistance)
    (bind _output_get (LocalVariables|SetDirection (Math|Vector|Normalize (- (Transformation|GetActorLocation (Variables|Default|GetTarget)) (Transformation|GetActorLocation)))))
    (Transformation|SetActorLocation (+ (Transformation|GetActorLocation) (* _output_get (* Speed Delta))) false false)
    (else
      (Default|GetAttackHit (Variables|Default|GetTarget) (Variables|Default|GetDamage))
      (Actor|DestroyActor))))