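; Bear unit character for Cardience that picks an opponent or player skeletal mesh on BeginPlay, rotating the root when it is the opponent's.
; Animation functions play attack, run and idle clips as loops directly on the mesh, while the hit function is empty with its impact clip disconnected.
; LaunchAttack locks movement, calls Attack and plays the attack animation once the target is reached, otherwise it unlocks movement.
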(event EventBeginPlay
  (CallFunction|Initialise)
  (if (Variables|Default|GetIsOpponent)
    (Transformation|SetRelativeRotation (Variables|Default|GetDefaultSceneRoot) "0,90.000000, 0" false false)
    (Class|SkinnedMeshComponent|SetSkeletalMesh (Variables|Default|GetSkeletalMesh) (Variables|Default|GetOpponentSkeletalMesh) true)
    (else
      (Class|SkinnedMeshComponent|SetSkeletalMesh (Variables|Default|GetSkeletalMesh) (Variables|Default|GetPlayerSkeletalMesh) true))))

(fn ConstructionScript)

(fn PlayAttackAnimation
  (Components|Animation|PlayAnimation (Variables|Default|GetSkeletalMesh) "/Game/Cardience/CardienceCharacters/Gladiator_bear/animation/anim_atak_2.anim_atak_2" true)
  (Development|PrintString "Hello"))

(fn PlayHitAnimation)

(fn PlayMoveAnimation
  (Components|Animation|PlayAnimation (Variables|Default|GetSkeletalMesh) "/Game/Cardience/CardienceCharacters/Gladiator_bear/animation/anim_run.anim_run" true))

(fn PlayIdleAnimation
  (Components|Animation|PlayAnimation (Variables|Default|GetSkeletalMesh) "/Game/Cardience/CardienceCharacters/Gladiator_bear/Demo/Mannequin/Animations/Anim_ThirdPersonIdle.Anim_ThirdPersonIdle" true))

(fn LaunchAttack
  (if (Variables|Default|GetHasReachedTarget?)
    (CallFunction|ManageMovementLock true)
    (CallFunction|Attack)
    (CallFunction|PlayAttackAnimation)
    (Variables|Default|SetHasReachedTarget? false)
    (else
      (CallFunction|ManageMovementLock false))))